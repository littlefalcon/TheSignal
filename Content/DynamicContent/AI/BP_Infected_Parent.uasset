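; Parent Blueprint for infected AI enemies that hear noises, melee the player and drop loot.
; Socket-attached hitboxes feed HitResponse, scaling projectile damage by body part and draining stand strength to trigger staggers.
; Surviving projectile hits and heard noises update the blackboard; projectile death unpossesses the controller, spawns drops, notifies GameManager and later destroys the actor.
; Melee hits lower health and stand strength but only log death.
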(event OnComponentBeginOverlap(Col_RightUpperArm)
  (params (OverlappedComponent :type Primitive%20Component%20Object%20Reference) (OtherActor :type Actor%20Object%20Reference) (OtherComp :type Primitive%20Component%20Object%20Reference) (OtherBodyIndex :type Integer) (bFromSweep :type Boolean) (SweepResult :type Hit%20Result%20Structure%20%28by%20ref%29))
  ;[1 1 1] Hit Mechanic
  (Utilities|HitResponse OtherActor 1.5 SweepResult "RUpperArm"))

(event OnComponentBeginOverlap(Col_LeftLowerArm)
  (params (OverlappedComponent :type Primitive%20Component%20Object%20Reference) (OtherActor :type Actor%20Object%20Reference) (OtherComp :type Primitive%20Component%20Object%20Reference) (OtherBodyIndex :type Integer) (bFromSweep :type Boolean) (SweepResult :type Hit%20Result%20Structure%20%28by%20ref%29))
  ;[1 1 1] Hit Mechanic
  (Utilities|HitResponse OtherActor 1.5 SweepResult "LLowerArm"))

(event OnComponentBeginOverlap(Col_RightLowerArm)
  (params (OverlappedComponent :type Primitive%20Component%20Object%20Reference) (OtherActor :type Actor%20Object%20Reference) (OtherComp :type Primitive%20Component%20Object%20Reference) (OtherBodyIndex :type Integer) (bFromSweep :type Boolean) (SweepResult :type Hit%20Result%20Structure%20%28by%20ref%29))
  ;[1 1 1] Hit Mechanic
  (Utilities|HitResponse OtherActor 1.5 SweepResult "RLowerArm"))

(event OnComponentBeginOverlap(Col_Body)
  (params (OverlappedComponent :type Primitive%20Component%20Object%20Reference) (OtherActor :type Actor%20Object%20Reference) (OtherComp :type Primitive%20Component%20Object%20Reference) (OtherBodyIndex :type Integer) (bFromSweep :type Boolean) (SweepResult :type Hit%20Result%20Structure%20%28by%20ref%29))
  ;[1 1 1] Hit Mechanic
  (Utilities|HitResponse OtherActor 1.0 SweepResult "BODY"))

(event OnComponentBeginOverlap(Col_Weapon)
  (params (OverlappedComponent :type Primitive%20Component%20Object%20Reference) (OtherActor :type Actor%20Object%20Reference) (OtherComp :type Primitive%20Component%20Object%20Reference) (OtherBodyIndex :type Integer) (bFromSweep :type Boolean) (SweepResult :type Hit%20Result%20Structure%20%28by%20ref%29))
  (bind _asbp_player (Utilities|Casting|CastToBP_Player OtherActor))
  (if (Variables|Default|GetAllowMelee)
    (Default|TakeDamage _asbp_player (Variables|Default|GetWeaponDamage))
    (Variables|Default|SetAllowMelee false)
    (Camera|PlayWorldCameraShake "/Game/DynamicContent/Player/CS_HitbyInfected.CS_HitbyInfected_C" (Transformation|GetWorldLocation (Variables|Default|GetCol_Weapon)) 0.0 1e+02)))

(event OnComponentBeginOverlap(Col_Head)
  (params (OverlappedComponent :type Primitive%20Component%20Object%20Reference) (OtherActor :type Actor%20Object%20Reference) (OtherComp :type Primitive%20Component%20Object%20Reference) (OtherBodyIndex :type Integer) (bFromSweep :type Boolean) (SweepResult :type Hit%20Result%20Structure%20%28by%20ref%29))
  ;[1 1 1] Hit Mechanic
  (Utilities|HitResponse OtherActor 1.5 SweepResult "HEAD"))

(event OnComponentBeginOverlap(Col_LeftUpperArm)
  (params (OverlappedComponent :type Primitive%20Component%20Object%20Reference) (OtherActor :type Actor%20Object%20Reference) (OtherComp :type Primitive%20Component%20Object%20Reference) (OtherBodyIndex :type Integer) (bFromSweep :type Boolean) (SweepResult :type Hit%20Result%20Structure%20%28by%20ref%29))
  ;[1 1 1] Hit Mechanic
  (Utilities|HitResponse OtherActor 1.5 SweepResult "LUpperArm"))

(event OnComponentBeginOverlap(Col_LeftUpperLeg)
  (params (OverlappedComponent :type Primitive%20Component%20Object%20Reference) (OtherActor :type Actor%20Object%20Reference) (OtherComp :type Primitive%20Component%20Object%20Reference) (OtherBodyIndex :type Integer) (bFromSweep :type Boolean) (SweepResult :type Hit%20Result%20Structure%20%28by%20ref%29))
  ;[1 1 1] Hit Mechanic
  (Utilities|HitResponse OtherActor 0.8 SweepResult "LUpperLeg"))

(event OnComponentBeginOverlap(Col_RightUpperLeg)
  (params (OverlappedComponent :type Primitive%20Component%20Object%20Reference) (OtherActor :type Actor%20Object%20Reference) (OtherComp :type Primitive%20Component%20Object%20Reference) (OtherBodyIndex :type Integer) (bFromSweep :type Boolean) (SweepResult :type Hit%20Result%20Structure%20%28by%20ref%29))
  ;[1 1 1] Hit Mechanic
  (Utilities|HitResponse OtherActor 0.8 SweepResult "RUpperLeg"))

(event OnComponentBeginOverlap(Col_RightLowerLeg)
  (params (OverlappedComponent :type Primitive%20Component%20Object%20Reference) (OtherActor :type Actor%20Object%20Reference) (OtherComp :type Primitive%20Component%20Object%20Reference) (OtherBodyIndex :type Integer) (bFromSweep :type Boolean) (SweepResult :type Hit%20Result%20Structure%20%28by%20ref%29))
  ;[1 1 1] Hit Mechanic
  (Utilities|HitResponse OtherActor 0.8 SweepResult "RLowerLeg"))

(event OnComponentBeginOverlap(Col_LeftLowerLeg)
  (params (OverlappedComponent :type Primitive%20Component%20Object%20Reference) (OtherActor :type Actor%20Object%20Reference) (OtherComp :type Primitive%20Component%20Object%20Reference) (OtherBodyIndex :type Integer) (bFromSweep :type Boolean) (SweepResult :type Hit%20Result%20Structure%20%28by%20ref%29))
  ;[1 1 1] Hit Mechanic
  (Utilities|HitResponse OtherActor 0.8 SweepResult "LLowerLeg"))

(event OnHearNoise(PawnSensing)
  (params (Instigator :type Pawn%20Object%20Reference) (Location :type Vector%20%28by%20ref%29 :default "0, 0, 0") (Volume :type Float%20%28single-precision%29))
  (bind _returnvalue (AI|GetBlackboard 0))
  (if (not (Variables|Default|GetAnim_IsDead))
    (Variables|Default|SetSoundMaker Instigator)
    (bind _output_get (Variables|Default|SetSoundLocation Location))
    (AI|Components|Blackboard|SetValueasVector _returnvalue (Utilities|Name|MakeLiteralName "SoundLocation") _output_get)
    (AI|Components|Blackboard|SetValueasBool _returnvalue (Utilities|Name|MakeLiteralName "IsHear") true)))

(event Custom|Run
  (Variables|/Script/Engine.CharacterMovementComponent|SetMaxWalkSpeed (Variables|Character|GetCharacterMovement) 3e+02))

(event Custom|HitbyMelee
  (params (Damage :type Float%20%28single-precision%29) (StuntAmount :type Float%20%28single-precision%29))
  ;[1 1 1] Hit Mechanic
  (Utilities|FlowControl|DoOnce false :!label _label
    (:Completed
      (Variables|Default|SetHealth (- (Variables|Default|GetHealth) Damage))
      (bind _output_get (Variables|Default|SetCurrentStandStrength (- (Variables|Default|GetCurrentStandStrength) StuntAmount)))
      (if (<= _output_get 0.0)
        (Utilities|SpeedDebug "INFECTED  DOWN" (Utilities|String|ToString(Float) (- (Variables|Default|GetCurrentStandStrength) StuntAmount)) "(R=0.000000,G=1.000000,B=0.048421,A=1.000000)" true)
        (Variables|Default|SetAnim_IsHit true)
        (Variables|Default|SetCurrentStandStrength (Variables|Default|GetStandStrength))
        (else
          (Utilities|SpeedDebug "INFECTED NOT DOWN" (Utilities|String|ToString(Float) (- (Variables|Default|GetCurrentStandStrength) StuntAmount)) "(R=0.520833,G=0.000000,B=0.000000,A=1.000000)" false)))
      (if (< (Variables|Default|GetHealth) 0.0)
        (Utilities|SpeedDebug "INFECTED DEAD" "" "(R=0.000000,G=1.000000,B=0.048421,A=1.000000)" true)
        (else
          (Utilities|SpeedDebug "INFECTED STILL NOT DEAD" "" "(R=0.520833,G=0.000000,B=0.000000,A=1.000000)" true)))
      (Utilities|FlowControl|Delay 0.2)
      (goto _label Reset))))

(event Custom|Walk
  (Variables|/Script/Engine.CharacterMovementComponent|SetMaxWalkSpeed (Variables|Character|GetCharacterMovement) 3e+02))

(event Custom|Attack
  (bind _output_get (Variables|Default|SetAnim_IsAttack true))
  (Utilities|SpeedDebug "ATTACK" (Utilities|String|ToString(Boolean) _output_get) "(R=0.000000,G=1.000000,B=0.958144,A=1.000000)" true))

(event Custom|EnableMeleeAttack
  (Variables|Default|SetAllowMelee true))

(event Custom|On%20Spawned
  (Default|OnSpawned (stale EventBeginPlay _output_get))
  (Variables|/Script/Engine.CharacterMovementComponent|SetMaxWalkSpeed (Variables|Character|GetCharacterMovement) 0.0))

(event EventBeginPlay
  (bind _asinfected_controller (Utilities|Casting|CastToInfectedController (AI|GetAIController self)))
  (bind _output_get (Variables|Default|SetInfectedController _asinfected_controller))
  (if (Variables|Default|GetCustomSpawn)
    (Variables|Default|SetSpawnAreaTag (Variables|Default|GetCustomSpawnTag))
    (CallFunction|OnSpawned)
    (Variables|Default|SetCurrentStandStrength (Variables|Default|GetStandStrength))))

(fn ConstructionScript
  ;[1 1 1] Weapon
  (CallFunction|AttachHitBox (Variables|Default|GetCol_Weapon) "Col_Weapon")
  ;[1 1 1] HeadBody
  (CallFunction|AttachHitBox (Variables|Default|GetCol_Head) "Col_Head")
  (CallFunction|AttachHitBox (Variables|Default|GetCol_Body) "Col_Body")
  ;[1 1 1] Arm
  (CallFunction|AttachHitBox (Variables|Default|GetCol_LeftUpperArm) "Col_LeftUpperArm")
  (CallFunction|AttachHitBox (Variables|Default|GetCol_LeftLowerArm) "Col_LeftLowerArm")
  (CallFunction|AttachHitBox (Variables|Default|GetCol_RightUpperArm) "Col_RightUpperArm")
  (CallFunction|AttachHitBox (Variables|Default|GetCol_RightLowerArm) "Col_RightLowerArm")
  ;[1 1 1] Leg
  (CallFunction|AttachHitBox (Variables|Default|GetCol_LeftUpperLeg) "Col_LeftUpperLeg")
  (CallFunction|AttachHitBox (Variables|Default|GetCol_LeftLowerLeg) "Col_LeftLowerLeg")
  (CallFunction|AttachHitBox (Variables|Default|GetCol_RightUpperLeg) "Col_RightUpperLeg")
  (CallFunction|AttachHitBox (Variables|Default|GetCol_RightLowerLeg) "Col_RightLowerLeg"))

(fn GetSpawnArea
  (bind _spawnareatag (Variables|Default|GetSpawnAreaTag))
  (Utilities|SpeedDebug :TOP (Utilities|String|ToString(Name) _spawnareatag) :ShowDebug true)
  (return _spawnareatag))

(fn PlayAttackAnimation
  (params (InfectedActor :type Skeletal%20Mesh%20Component%20Object%20Reference) (NewAnimToPlay :type Animation%20Asset%20Object%20Reference))
  (Variables|Default|SetIsAttack true))

(fn AttachHitBox
  (params (HitBox :type Scene%20Component%20Object%20Reference) (SocketName :type Name))
  (Transformation|AttachComponentToComponent HitBox (Variables|Character|GetMesh) SocketName "KeepRelative" "KeepRelative" "KeepRelative" true))