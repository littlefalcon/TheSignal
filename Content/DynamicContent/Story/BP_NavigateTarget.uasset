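; Story navigation target actor that marks a location and can advance the story when the player reaches it.
; On BeginPlay it sets the widget text, hides both marker meshes and widget, and enables trigger queries only if InstantNextToStory is set.
; Player overlap then logs debug text and passes StoryMessage to the game mode's SetNextToStory.
; SetHiddenMarker toggles marker and widget visibility separately, and PlaySoundLoop plays the quest sound at the actor.
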(event OnComponentBeginOverlap(Trigger)
  (params (OverlappedComponent :type Primitive%20Component%20Object%20Reference) (OtherActor :type Actor%20Object%20Reference) (OtherComp :type Primitive%20Component%20Object%20Reference) (OtherBodyIndex :type Integer) (bFromSweep :type Boolean) (SweepResult :type Hit%20Result%20Structure%20%28by%20ref%29))
  (Utilities|Casting|CastToBP_Player OtherActor)
  (Utilities|SpeedDebug "STORY TRIGGER TOUCHED PLAYER" "" "(R=0.000000,G=1.000000,B=0.048421,A=1.000000)" true)
  (if (Variables|Default|GetInstantNextToStory)
    (Default|SetNexttoStory (CallFunction|GetGameMode) (Variables|Default|GetStoryMessage))))

(event Custom|Event%20PlaySound%20Loop
  (Audio|PlaySoundatLocation (Variables|Default|GetQuestSound) (Transformation|GetWorldLocation (Variables|Default|GetDefaultSceneRoot1))))

(event EventBeginPlay
  (bind _trigger (Variables|Default|GetTrigger))
  (if (Variables|Default|GetInstantNextToStory)
    (Collision|SetCollisionEnabled _trigger "QueryOnly")
    (else
      (Collision|SetCollisionEnabled _trigger "NoCollision")))
  (Default|SetText (Variables|Default|GetInteractWidget) (Variables|Default|GetTEXT))
  (CallFunction|SetHiddenMarker true true))

(event Collision|EventActorBeginOverlap
  (params (OtherActor :type Actor%20Object%20Reference)))

(event EventTick
  (params (DeltaSeconds :type Float%20%28single-precision%29)))

(fn ConstructionScript)

(fn SetHiddenMarker
  (params (HiddenMarker :type Boolean) (HiddenWidget :type Boolean))
  (Development|SetHiddeninGame (Variables|Default|GetX1) HiddenMarker false)
  (Development|SetHiddeninGame (Variables|Default|GetX2) HiddenMarker false)
  (Development|SetHiddeninGame (Variables|Default|GetInteractWidget) HiddenWidget false))