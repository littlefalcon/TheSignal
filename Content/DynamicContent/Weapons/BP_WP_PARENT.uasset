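; Base weapon Blueprint managing stats, magazine and overheat, with empty Fire and AssignProjectile events.
; AssembleWeapon loads stats from a data table row named by weapon type and MK variant, while ConstructWeapon hardcodes DoorCutterMK0.
; BeginPlay fills the magazine and converts fire rate.
; DeceaseClip either checks ammo or spends a round and adds heat, failing on depletion or overheat; Tick cools heat over time.
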(event Custom|DeceaseMagazine)

(event Custom|AssignProjectile)

(event Custom|Fire)

(event EventBeginPlay
  (CallFunction|SetupWeapon))

(event EventTick
  (params (DeltaSeconds :type Float%20%28single-precision%29))
  (if (> (Variables|Mechanic|GetCurrentOverheat) 0.0)
    (Variables|Mechanic|SetCurrentOverheat (- (Variables|Mechanic|GetCurrentOverheat) (* DeltaSeconds 1e+01)))))

(fn ConstructionScript)

(fn DeceaseClip
  (params (CheckAmmo :type Boolean))
  (bind _returnvalue (Utilities|OverheatResult))
  ;[1 1 1] Check or Fire Ammo
  (if CheckAmmo
    (Utilities|CheckAmmo
      (:Have
        _)
      (:Deplete
        (return false)))
    (else
      ;[1 1 1] Overheat Condition Check
      (if (>= _returnvalue (Variables|Mechanic|GetMaxOverheat))
        (return false)
        (else
          (bind _output_get (Variables|Mechanic|SetCurrentOverheat _returnvalue))
          ;[1 1 1] Decease Ammo Condition Check
          (if (> (Variables|DynamicVariable|GetCurrentMagazineCapacity) 0.0)
            (bind _output_get_2 (Variables|DynamicVariable|SetCurrentMagazineCapacity (- (Variables|DynamicVariable|GetCurrentMagazineCapacity) 1.0)))
            (Utilities|FastDebug :TOP (Utilities|String|ToString(Float) _output_get_2) :MID "  < Current Ammo | Heat >  " :BOT (Utilities|String|ToString(Float) _output_get))
            ;[1 1 1] IS OVERHEAT?
            (if (>= (Variables|Mechanic|GetCurrentOverheat) (Variables|Mechanic|GetMaxOverheat))
              (return false)
              (else
                _))
            (else
              (bind _output_get_3 (Variables|DynamicVariable|SetCurrentMagazineCapacity 0.0))
              (Utilities|FastDebug :TOP "AMMO DEPLETE" :MID (Utilities|String|ToString(Float) _output_get_3))
              (return false)))))))
  (return true))

(fn SetupWeapon
  (Variables|DynamicVariable|SetCurrentMagazineCapacity (Variables|General|GetMagazineCapacity))
  (CallFunction|ConvertFireRate))

(fn ConvertFireRate
  (bind _output_get (Variables|General|SetFireRate (Utilities|ConvertFirerate (Variables|General|GetFireRate))))
  (Utilities|SpeedDebug :TOP (Utilities|String|ToString(Float) _output_get))
  (return))

(fn UpdateWeaponVariant
  (bind _weaponvariant (Variables|Default|GetWeaponVariant))
  (bind _returnvalue (>= _weaponvariant 0))
  (Utilities|SpeedDebug (Utilities|String|ToString(Integer) _weaponvariant) "(R=0.000000,G=1.000000,B=0.939229,A=1.000000)" true)
  (if _returnvalue
    (CallFunction|AssembleWeapon _weaponvariant))
  (return _returnvalue))

(fn AssembleWeapon
  (params (WeaponVariant :type Integer))
  ;[1 1 1] INIT DEBUG
  (Utilities|FastDebug "Initialize Construct " (Utilities|GetDisplayName self) "" "" "" "(R=0.000000,G=1.000000,B=0.958144,A=1.000000)" true)
  ;[1 1 1] SELECTING WEAPON SETTING FROM INSTANCE
  (bind _returnvalue (Utilities|GetDataTableRow "/Game/DynamicContent/Weapons/WeaponDataTable.WeaponDataTable" (Utilities|String|StringToName (Utilities|String|Append (Utilities|String|EnumtoString (Variables|Default|GetWeaponInstance)) "MK" (Utilities|String|ToString(Integer) WeaponVariant))))
    (:then
      (Variables|Default|SetWeaponInformation _returnvalue)
      ;[1 1 1] ASSIGN WEAPON STATS
      (Utilities|FlowControl|Sequence
        (:then_0
          (bind _output_get (Variables|General|SetDamage (.Damage (Utilities|Struct|BreakWeaponStructure (Variables|Default|GetWeaponInformation))))))
        (:then_1
          (bind _output_get_2 (Variables|General|SetFireRate (.FireRate (Utilities|Struct|BreakWeaponStructure (Variables|Default|GetWeaponInformation))))))
        (:then_2
          (bind _output_get_3 (Variables|Mechanic|SetFireRange (.EffectiveRange (Utilities|Struct|BreakWeaponStructure (Variables|Default|GetWeaponInformation))))))
        (:then_3
          (bind _output_get_4 (Variables|General|SetReloadSpeed (.ReloadTime (Utilities|Struct|BreakWeaponStructure (Variables|Default|GetWeaponInformation))))))
        (:then_4
          (bind _output_get_5 (Variables|General|SetMagazineCapacity (.MagazineClip (Utilities|Struct|BreakWeaponStructure (Variables|Default|GetWeaponInformation))))))
        (:then_5
          (bind _output_get_6 (Variables|General|SetBatteryConsume (.BatteryConsumption (Utilities|Struct|BreakWeaponStructure (Variables|Default|GetWeaponInformation))))))
        (:then_6
          (bind _output_get_7 (Variables|Mechanic|SetOverheatRate (.OverheatRate (Utilities|Struct|BreakWeaponStructure (Variables|Default|GetWeaponInformation))))))
        (:then_7
          ;[1 1 1] PRINT
          (Development|PrintString (Utilities|String|Append "DMG>[ " (Utilities|String|ToString(Float) _output_get) "]FRATE>[ " (Utilities|String|ToString(Float) _output_get_2) "]FRNG>[" (Utilities|String|ToString(Float) _output_get_3) "]RELOAD>[" (Utilities|String|ToString(Float) _output_get_4) "]CLIP>[" (Utilities|String|ToString(Float) _output_get_5) "]BATCS>[" (Utilities|String|ToString(Float) _output_get_6) "]HRATE>[" (Utilities|String|ToString(Float) _output_get_7) "]") false true "(R=0.000000,G=1.000000,B=0.048421,A=1.000000)")
          (return))))
    (:RowNotFound
      ;[1 1 1] DATA TABLE NOT FOUND
      (Utilities|FastDebug "Weapon " (Utilities|GetDisplayName self) " Not Found a Data!" "" "" "(R=0.000000,G=1.000000,B=0.958144,A=1.000000)" true)
      (return))))