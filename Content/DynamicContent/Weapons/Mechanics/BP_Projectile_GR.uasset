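; Gauss Rifle projectile Blueprint that takes its stats from the player's weapon when spawned.
; BeginPlay casts player character 0, fetches its Gauss Rifle and passes it to SetProjectileInfo before calling parent BeginPlay, which is skipped if the cast fails.
; SetProjectileInfo copies Damage, sets StableTime to FireRange divided by ConvertFireRangeToTime, and shows that value as debug output.
; FXGetDamageGR is an empty stub.
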(event EventBeginPlay
  (bind _asbp_player (Utilities|Casting|CastToBP_Player (Game|GetPlayerCharacter 0)))
  (bind _asbp_weapon (Default|FXCasttoGaussRifle _asbp_player))
  (CallFunction|SetProjectileInfo _asbp_weapon)
  (|CallParentFunction))

(event Collision|EventActorBeginOverlap
  (params (OtherActor :type Actor%20Object%20Reference)))

(event EventTick
  (params (DeltaSeconds :type Float%20%28single-precision%29)))

(fn ConstructionScript
  (|CallParentFunction))

(fn FXGetDamageGR
  (return))

(fn SetProjectileInfo
  (params (BP_Weapon :type BP%20WP%20PARENT%20Object%20Reference))
  (bind _constant (Utilities|ConvertFireRangetoTime))
  (bind _firerange (Variables|/Game/DynamicContent/Weapons/BP_WP_PARENT.BP_WP_PARENT_C|GetFireRange BP_Weapon))
  (bind _returnvalue (/ _firerange _constant))
  (Variables|Default|SetDamage (Variables|/Game/DynamicContent/Weapons/BP_WP_PARENT.BP_WP_PARENT_C|GetDamage BP_Weapon))
  (Utilities|SpeedDebug :TOP (Utilities|String|ToString(Float) _returnvalue) :ShowDebug true)
  (Variables|Default|SetStableTime _returnvalue))