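; Projectile Blueprint for the Door Cutter weapon, a child class that configures itself from the player's weapon on spawn.
; On BeginPlay it gets the Door Cutter through BP_Player and copies its Damage.
; It derives StableTime by dividing the weapon's FireRange by ConvertFireRangeToTime, also sending that value to SpeedDebug.
; The parent BeginPlay runs last, after these values are set, and only if the player cast succeeds.
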(event EventBeginPlay
  (bind _asbp_player (Utilities|Casting|CastToBP_Player (Game|GetPlayerCharacter 0)))
  (bind _asbp_weapon (Default|FXCasttoDoorCutter _asbp_player))
  (Variables|Default|SetDamage (Variables|/Game/DynamicContent/Weapons/BP_WP_PARENT.BP_WP_PARENT_C|GetDamage _asbp_weapon))
  (Utilities|SpeedDebug :TOP (Utilities|String|ToString(Float) (/ (Variables|/Game/DynamicContent/Weapons/BP_WP_PARENT.BP_WP_PARENT_C|GetFireRange _asbp_weapon) (Utilities|ConvertFireRangetoTime))))
  (Variables|Default|SetStableTime (/ (Variables|/Game/DynamicContent/Weapons/BP_WP_PARENT.BP_WP_PARENT_C|GetFireRange _asbp_weapon) (Utilities|ConvertFireRangetoTime)))
  (|CallParentFunction))

(fn ConstructionScript
  (|CallParentFunction))