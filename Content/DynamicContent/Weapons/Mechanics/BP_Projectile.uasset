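; BP_Projectile is a weapon projectile whose damage falls off over its lifetime before it destroys itself.
; After an initial StableTime delay, a BeginPlay delay loop divides Damage by FalloffDamageMultiplier and counts DestroyTime down until the actor is destroyed.
; StableTime also paces each loop pass, and a helper can set it to zero.
; A duplicate fixed-delay loop is left unconnected.
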(event EventBeginPlay
  (Utilities|StartDamageFalling)
  (Utilities|DeceaseDamage (Variables|Default|GetFalloffDamageMultiplier) :!label _label)
  (Utilities|DestroyCondition
    (:TRUE
      (Actor|DestroyActor))
    (:FALSE
      (Utilities|FlowControl|Delay (Variables|Default|GetStableTime))
      (goto _label))))

(fn ConstructionScript)