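; World pickup prop for the Door Cutter (DC) weapon, collected by the player.
; On BeginPlay it creates a pickup text widget and binds to the player's AssignPickupItem dispatcher; trigger overlaps show or hide the prompt and track range.
; A pickup event while in range and allowed destroys the prop, plays a sound, notifies the OpenWorldMode actor and sets the player's HasDCGun flag.
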(event OnComponentBeginOverlap(Trigger)
  (params (OverlappedComponent :type Primitive%20Component%20Object%20Reference) (OtherActor :type Actor%20Object%20Reference) (OtherComp :type Primitive%20Component%20Object%20Reference) (OtherBodyIndex :type Integer) (bFromSweep :type Boolean) (SweepResult :type Hit%20Result%20Structure%20%28by%20ref%29))
  (Utilities|Casting|CastToBP_Player OtherActor)
  (UserInterface|Viewport|AddtoViewport (Variables|Default|GetPickupTextReference) 0)
  (Variables|Default|SetIsInRange true))

(event OnComponentEndOverlap(Trigger)
  (params (OverlappedComponent :type Primitive%20Component%20Object%20Reference) (OtherActor :type Actor%20Object%20Reference) (OtherComp :type Primitive%20Component%20Object%20Reference) (OtherBodyIndex :type Integer))
  (Utilities|Casting|CastToBP_Player OtherActor)
  (Widget|RemovefromParent (Variables|Default|GetPickupTextReference))
  (Variables|Default|SetIsInRange false))

(event Custom|Event_PickupItem
  (if (and (Variables|Default|GetIsInRange) (Variables|Default|GetAllowToPickup))
    (CallFunction|AddNewWeapontoPlayer)))

(event EventBeginPlay
  ;[1 1 1] Event Begin Play
  (bind _returnvalue (UserInterface|CreateWidget "/Game/DynamicContent/Engine/Inventory/PickupText.PickupText_C" (Game|GetPlayerController 0)))
  (Variables|Default|SetPickupTextReference _returnvalue)
  (Variables|/Game/DynamicContent/Engine/Inventory/PickupText.PickupText_C|SetPickupActor (Variables|Default|GetPickupTextReference) self)
  (Variables|/Game/DynamicContent/Engine/Inventory/PickupText.PickupText_C|SetPickupText (Variables|Default|GetPickupTextReference) "Door Cutter")
  (bind _asbp_player (Utilities|Casting|CastToBP_Player (Game|GetPlayerCharacter 0)))
  (bind _output_get (Variables|Default|SetCharacterReference _asbp_player))
  (EventDispatchers|AssignPickupItem _output_get (delegate Custom|Event_PickupItem)))

(fn ConstructionScript)

(fn AddNewWeapontoPlayer
  (Actor|DestroyActor)
  (Audio|PlaySound2D "/Game/DynamicContent/Sounds/Power_Up_Gained.Power_Up_Gained")
  (bind _outactors (Actor|GetAllActorsOfClass "/Game/DynamicContent/Engine/OpenWorldMode.OpenWorldMode_C"))
  (Default|PickedupDoorCutter (Utilities|Array|Get(acopy) _outactors))
  (bind _asbp_player (Utilities|Casting|CastToBP_Player (Game|GetPlayerCharacter 0)))
  (Variables|/Game/DynamicContent/Player/BP_Player.BP_Player_C|SetHasDCGun _asbp_player true))