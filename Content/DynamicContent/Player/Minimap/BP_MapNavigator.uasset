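; BP_MapNavigator is a minimap navigation actor that turns to point toward a tracked target.
; TrackTarget sets its rotation via FindArrowDirection, whose look-at math zeroes pitch to keep the arrow flat, though that node appears unconnected.
; Instead of using Tick, it loops through a 0.2-second Delay, writing player-to-target distance to the game mode's TrackDistance until StopTrack is set.
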(event Custom|TrackTarget
  (params (Target :type Actor%20Object%20Reference))
  (bind _asopen_world_mode (CallFunction|GetGameMode))
  (Transformation|SetActorRotation (Utilities|FindArrowDirection (Transformation|GetWorldLocation (Variables|/Script/Engine.Actor|GetRootComponent Target))) :!label _label)
  (Utilities|FlowControl|Delay 0.2)
  (Variables|/Game/DynamicContent/Engine/OpenWorldMode.OpenWorldMode_C|SetTrackDistance _asopen_world_mode (Transformation|GetDistanceTo (Game|GetPlayerCharacter 0) Target))
  (if (not (Variables|/Game/DynamicContent/Engine/OpenWorldMode.OpenWorldMode_C|GetStopTrack _asopen_world_mode))
    (goto _label)))

(event EventBeginPlay)

(event Collision|EventActorBeginOverlap
  (params (OtherActor :type Actor%20Object%20Reference)))

(event EventTick
  (params (DeltaSeconds :type Float%20%28single-precision%29)))

(fn ConstructionScript)